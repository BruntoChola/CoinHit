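; Test actor that uses the IA_Jump Enhanced Input action to recolor its cube and spawn copies of its own class.
; Tick repeatedly enables input from player 0 and adds the mapping context, rather than doing so once at BeginPlay.
; Pressing swaps the Cube material and prints a debug string.
; Releasing spawns a Test_spawn at a stored position, which starts at a fixed point and steps along Y after each spawn.
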(event Input|EnhancedActionEvents|EnhancedInputActionIA_Jump
  (params (ActionValue :type Boolean) (ElapsedSeconds :type Float%20%28double-precision%29) (TriggeredSeconds :type Float%20%28double-precision%29) (InputAction :type Input%20Action%20Object%20Reference :default "/Game/Input/Actions/IA_Jump.IA_Jump"))
  (:Started
    (Development|PrintString "color change triggered")
    (Rendering|Material|SetMaterial (Variables|Default|GetCube) 0 (Variables|Default|GetMaterial_1)))
  (:Completed
    (Game|SpawnActorfromClass "test_spawn_C" (Math|Conversions|ToTransform(Vector) (Variables|Default|GetPosition)) "Undefined" "MultiplyWithRoot" 0 0)
    (Variables|Default|SetPosition (+ (Variables|Default|GetPosition) "0.000000,100.000000,0.000000"))))

(event EventBeginPlay
  (Variables|Default|SetPosition "0.000000,0.000000,50.000000"))

(event Collision|EventActorBeginOverlap
  (params (OtherActor :type Actor%20Object%20Reference)))

(event EventTick
  (params (DeltaSeconds :type Float%20%28single-precision%29))
  (bind _returnvalue (Game|GetPlayerController 0))
  (Input|EnableInput _returnvalue)
  (bind _asplayer_controller (Utilities|Casting|CastToPlayerController _returnvalue))
  (Input|AddMappingContext (PlayerController|LocalPlayerSubsystems|GetEnhancedInputLocalPlayerSubsystem _asplayer_controller) "/Game/Blueprints/NewInputMappingContext.NewInputMappingContext" 0 "(bIgnoreAllPressedKeysUntilRelease=True,bForceImmediately=False,bNotifyUserSettings=False)"))

(fn ConstructionScript)