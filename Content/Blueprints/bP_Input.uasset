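; bP_Input is an actor Blueprint that appears to test input handling.
; On BeginPlay it enables input from player 0, then the I key swaps a material on the referenced Gun's RoseFantasyWorldDemon between a pressed and a released look.
; An Enhanced Input jump action prints a debug string while ongoing.
; The code adding the mapping context is unconnected and never runs.
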(event Input|EnhancedActionEvents|EnhancedInputActionIA_Jump
  (params (ActionValue :type Boolean) (ElapsedSeconds :type Float%20%28double-precision%29) (TriggeredSeconds :type Float%20%28double-precision%29) (InputAction :type Input%20Action%20Object%20Reference :default "/Game/Input/Actions/IA_Jump.IA_Jump"))
  (:Ongoing
    (Development|PrintString "Jump")))

(event EventBeginPlay
  (Input|EnableInput (Game|GetPlayerController 0)))

(event Collision|EventActorBeginOverlap
  (params (OtherActor :type Actor%20Object%20Reference)))

(event EventTick
  (params (DeltaSeconds :type Float%20%28single-precision%29)))

(event Input|KeyboardEvents|I
  (params (Key :type Key%20Structure :default "None"))
  (bind _gun (Variables|Default|GetGun))
  (bind _rose_fantasy_world___demon (Variables|/Game/Blueprints/BP_gun.BP_gun_C|Getrose_fantasy_world___demon _gun))
  (:Pressed
    (Rendering|Material|SetMaterial _rose_fantasy_world___demon 0 (Variables|Default|GetMaterial1)))
  (:Released
    (Rendering|Material|SetMaterial _rose_fantasy_world___demon 0 (Variables|Default|GetMaterial2))))

(fn ConstructionScript)