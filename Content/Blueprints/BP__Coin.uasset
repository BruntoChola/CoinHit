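; Coin pickup actor that spins in place and can be collected by either BP_ThirdPersonCharacter or BP_OPP.
; BeginPlay applies the coin material to the Ert component and adds a randomized starting rotation, then Tick keeps it turning through an eased local rotation.
; On overlap with Ert, it calls the collector's Collection, sets that character's max walk speed to a fixed value and destroys itself.
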(event OnComponentBeginOverlap(ert)
  (params (OverlappedComponent :type Primitive%20Component%20Object%20Reference) (OtherActor :type Actor%20Object%20Reference) (OtherComp :type Primitive%20Component%20Object%20Reference) (OtherBodyIndex :type Integer) (bFromSweep :type Boolean) (SweepResult :type Hit%20Result%20Structure%20%28by%20ref%29))
  (bind _asbp_third_person_character (Utilities|Casting|CastToBP_ThirdPersonCharacter OtherActor)
    (:then
      (Default|Collection _asbp_third_person_character 1)
      (Variables|/Script/Engine.CharacterMovementComponent|SetMaxWalkSpeed (Variables|/Script/Engine.Character|GetCharacterMovement _asbp_third_person_character) 6e+02)
      (Actor|DestroyActor))
    (:CastFailed
      (bind _asbp_opp (Utilities|Casting|CastToBP_OPP OtherActor))
      (Default|Collection _asbp_opp 1)
      (Variables|/Script/Engine.CharacterMovementComponent|SetMaxWalkSpeed (Variables|/Script/Engine.Character|GetCharacterMovement _asbp_opp) 6e+02)
      (Actor|DestroyActor))))

(event EventTick
  (params (DeltaSeconds :type Float%20%28single-precision%29))
  (bind _result (Math|Float|IncrementFloat DeltaSeconds)
    (:%20%20
      (Transformation|AddActorLocalRotation (Math|Interpolation|Ease "SinusoidalIn" _result "0.000000,1.000000,0.000000" "0.000000,5.000000,0.000000" true) false false))))

(event EventBeginPlay
  (Rendering|Material|SetMaterial (Variables|Default|Getert) 0 "/Game/materials/m_cooin_Inst.m_cooin_Inst")
  (Transformation|AddActorLocalRotation (Math|Interpolation|Ease :Function "Linear" :Alpha (Math|Conversions|ToFloat(Integer) (Math|Random|RandomInteger 360)) :A "0.000000,1.000000,0.000000") false false))

(fn ConstructionScript)